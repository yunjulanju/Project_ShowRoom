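; Showroom product display actor that shows a mannequin with product meshes added at runtime and offers preset camera views.
; On BeginPlay it counts DT_Acne_CameraPresets rows containing its ProductName, then applies the current `ProductName_Cam#` preset.
; While the showroom character is inside the Box, MoveCamNumber cycles presets with wraparound, and a timeline lerps the Camera's relative transform.
; MouseRotate spins the whole actor locally.
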(event `self.ReceiveBeginPlay`
  ; 스폰 될 때 ProductName에 값이 들어가는 타이밍과 비긴 플레이 타이밍이 맞지 않아서 이름이 널값이라 camera의  값을 찾지 못함. -> 타이밍 문제는 해결 스폰할 때 넣어버림. 근데 왜 같은 내용인데 못찾는 거임 -> Name으로 바꾸니까 인식 되고, 데이터 테이블 값 확인 안해서였음.
  (`self.Get GameraPresetLength`)
  (`self.ChangeCameraOffset` (`self.ProductName`) (`self.CamNumber`)))

(event `self.Box.OnComponentBeginOverlap`
  (params (OverlappedComponent :type "PrimitiveComponent Object Reference") (OtherActor :type "Actor Object Reference") (OtherComp :type "PrimitiveComponent Object Reference") (OtherBodyIndex :type Integer) (bFromSweep :type Boolean) (SweepResult :type "HitResult Structure (by ref)"))
  (cast `/Game/Blueprints/Character/ShowRoom/BP_ShowRoomCharacter` OtherActor)
  (set `self.bInPlayer` true))

(event `self.Box.OnComponentEndOverlap`
  (params (OverlappedComponent :type "PrimitiveComponent Object Reference") (OtherActor :type "Actor Object Reference") (OtherComp :type "PrimitiveComponent Object Reference") (OtherBodyIndex :type Integer))
  (set `self.bInPlayer` false))

(event `SetCameraOffset`
  (params (CurrentTransform :type "Transform Structure") (NewTransform :type "Transform Structure"))
  (bind (_direction _alpha) (`Timeline|MoveCamera` :!via `PlayFromStart`)
    (:`Update`
      (`SceneComponent.K2_SetRelativeTransform` (`self.Camera`) (`KismetMathLibrary.TLerp` CurrentTransform NewTransform _alpha) false false))))

(fn `ChangeCameraOffset`
  (params (ProductName :type Name) (CamNumber :type Integer))
  (bind _returnvalue (`|GetDataTableRow` "/Game/Blueprints/Datas/DataTable/Acne/DT_Acne_CameraPresets.DT_Acne_CameraPresets" (`KismetStringLibrary.Conv_StringToName` (`KismetStringLibrary.Concat_StrStr` (`KismetStringLibrary.Conv_NameToString` ProductName) "_Cam" (`KismetStringLibrary.Conv_IntToString` CamNumber))))
    (:`then`
      (bind (_viewname _location _rotation) (break `/Game/Blueprints/Datas/Struct/ST_Show_CameraPreset` _returnvalue))
      (bind _returnvalue_2 (`KismetMathLibrary.MakeTransform` _location _rotation))
      (if (not (== (`self.CurrentCameraTransform`) _returnvalue_2))
        (`self.SetCameraOffset` (`self.CurrentCameraTransform`) _returnvalue_2))
      (set `self.CurrentCameraTransform` _returnvalue_2))))

(fn `Get GameraPresetLength`
  (bind _outrownames (`DataTableFunctionLibrary.GetDataTableRowNames` "/Game/Blueprints/Datas/DataTable/Acne/DT_Acne_CameraPresets.DT_Acne_CameraPresets"))
  (for _array_element _outrownames
    (if (`KismetStringLibrary.Contains` (`KismetStringLibrary.Conv_NameToString` _array_element) (`KismetStringLibrary.Conv_NameToString` (`self.ProductName`)))
      (`/Engine/EditorBlueprintResources/StandardMacros.IncrementInt` (`self.CamLength`)))))

(fn `MouseRotate`
  (params (NewRotator :type "Rotator Structure"))
  (`self.K2_AddActorLocalRotation` NewRotator))

(fn `MoveCamNumber`
  (params (bIsRight :type Boolean))
  (bind _returnvalue (+ (`self.CamNumber`) 1))
  (bind _returnvalue_2 (- (`self.CamNumber`) 1))
  (if (`self.bInPlayer`)
    (if (`local.bIsRight`)
      (if (<= _returnvalue (`self.CamLength`))
        (set `self.CamNumber` _returnvalue)
        (else
          (set `self.CamNumber` (+ (- (`self.CamNumber`) (`self.CamLength`)) 1))))
      (elif (> _returnvalue_2 0)
        (set `self.CamNumber` _returnvalue_2)
        (else
          (set `self.CamNumber` (`self.CamLength`)))))
    (`self.ChangeCameraOffset` (`self.ProductName`) (`self.CamNumber`))))

(fn `SetProductInfo`
  (params (InMannequin :type "StaticMesh Object Reference") (InInteractionable :type Boolean) (Products :type "Array of /Game/Blueprints/Datas/Struct/ST_Transform Structure"))
  (`|ExecutionSequence`
    (:`then_0`
      (`StaticMeshComponent.SetStaticMesh` (`self.Mannequin`) InMannequin))
    (:`then_1`
      (set `self.bIsInteractionable` InInteractionable))
    (:`then_2`
      (for _array_element Products
        (bind _returnvalue (`AddComponent|NODE_AddStaticMeshComponent-1` :`RelativeTransform` (`.Transform_6_33D266764536582172C891A6AD269446` (break `/Game/Blueprints/Datas/Struct/ST_Transform` _array_element))))
        (`StaticMeshComponent.SetStaticMesh` _returnvalue (break `/Game/Blueprints/Datas/Struct/ST_Transform` _array_element))))))

(fn `UserConstructionScript`)