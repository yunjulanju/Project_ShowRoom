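; Showroom product actor that displays static or skeletal meshes with switchable camera presets and rotation.
; SetMeshes spawns mesh components from passed-in arrays, which MouseRotate and InitMeshRotate rotate or reset.
; A box overlap sets InPlayer, gating MoveCamNumber as it steps through presets counted by product-name matches in DT_Acne_CameraPresets.
; ChangeCameraOffset looks up rows named product plus "_Cam" and number, then a timeline blends the camera's relative transform.
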(event `self.Box.OnComponentBeginOverlap`
  (params (OverlappedComponent :type "PrimitiveComponent Object Reference") (OtherActor :type "Actor Object Reference") (OtherComp :type "PrimitiveComponent Object Reference") (OtherBodyIndex :type Integer) (bFromSweep :type Boolean) (SweepResult :type "HitResult Structure (by ref)"))
  (cast `/Game/Blueprints/Character/BP_Character` OtherActor)
  (set `self.In Player` true))

(event `self.Box.OnComponentEndOverlap`
  (params (OverlappedComponent :type "PrimitiveComponent Object Reference") (OtherActor :type "Actor Object Reference") (OtherComp :type "PrimitiveComponent Object Reference") (OtherBodyIndex :type Integer))
  (set `self.In Player` false))

(event `SetCameraOffset`
  (params (CurrentTransform :type "Transform Structure") (NewTransform :type "Transform Structure"))
  (bind (_direction _alpha) (`Timeline|Timeline` :!via `PlayFromStart`)
    (:`Update`
      (`SceneComponent.K2_SetRelativeTransform` (`self.Camera`) (`KismetMathLibrary.TLerp` CurrentTransform NewTransform _alpha) false false))))

(fn `ChangeCameraOffset`
  (params (ProductName :type Name) (CamNumber :type Integer))
  (bind _returnvalue (`|GetDataTableRow` "/Game/Blueprints/Datas/DataTable/Acne/DT_Acne_CameraPresets.DT_Acne_CameraPresets" (`KismetStringLibrary.Conv_StringToName` (`KismetStringLibrary.Concat_StrStr` (`KismetStringLibrary.Conv_NameToString` ProductName) "_Cam" (`KismetStringLibrary.Conv_IntToString` CamNumber))))
    (:`then`
      (bind (_viewname _location _rotation) (break `/Game/Blueprints/Datas/Struct/ShowRoom/ST_Show_CameraPreset` _returnvalue))
      (bind _returnvalue_2 (`KismetMathLibrary.MakeTransform` _location _rotation))
      (if (not (== (`self.Current Camera Transform`) _returnvalue_2))
        (`self.SetCameraOffset` (`self.Current Camera Transform`) _returnvalue_2))
      (set `self.Current Camera Transform` _returnvalue_2))))

(fn `Get GameraPresetLength`
  (bind _outrownames (`DataTableFunctionLibrary.GetDataTableRowNames` "/Game/Blueprints/Datas/DataTable/Acne/DT_Acne_CameraPresets.DT_Acne_CameraPresets"))
  (for _array_element _outrownames
    (if (`KismetStringLibrary.Contains` (`KismetStringLibrary.Conv_NameToString` _array_element) (`KismetStringLibrary.Conv_NameToString` (`self.ProductName`)))
      (`/Engine/EditorBlueprintResources/StandardMacros.IncrementInt` (`self.Cam Length`)))))

(fn `InitMeshRotate`
  (switch `/Game/Blueprints/Datas/Enum/E_MeshType` (`self.Mesh Type`)
    (:`NewEnumerator0`
      (for _array_element (`self.StaticMeshesComp`)
        (`SceneComponent.K2_SetRelativeRotation` :`self` _array_element)))
    (:`NewEnumerator1`
      (for _array_element_2 (`self.SkeletalMeshesComp`)
        (`SceneComponent.K2_SetRelativeRotation` :`self` _array_element_2)))))

(fn `MouseRotate`
  (params (NewRotator :type "Rotator Structure"))
  (switch `/Game/Blueprints/Datas/Enum/E_MeshType` (`self.Mesh Type`)
    (:`NewEnumerator0`
      (for _array_element (`self.StaticMeshesComp`)
        (`SceneComponent.K2_AddLocalRotation` _array_element (`local.NewRotator`) false false)))
    (:`NewEnumerator1`
      (for _array_element_2 (`self.SkeletalMeshesComp`)
        (`SceneComponent.K2_AddLocalRotation` _array_element_2 (`local.NewRotator`) false false)))))

(fn `MoveCamNumber`
  (params (bIsRight :type Boolean))
  (bind _returnvalue (+ (`self.Cam Number`) 1))
  (bind _returnvalue_2 (- (`self.Cam Number`) 1))
  (if (`self.In Player`)
    (if (`local.bIsRight`)
      (if (<= _returnvalue 0)
        (set `self.Cam Number` _returnvalue)
        (else
          (set `self.Cam Number` (+ (- (`self.Cam Number`) (`self.Cam Length`)) 1))))
      (elif (> _returnvalue_2 0)
        (set `self.Cam Number` _returnvalue_2)
        (else
          (set `self.Cam Number` (`self.Cam Length`)))))
    (`self.ChangeCameraOffset` (`self.ProductName`) (`self.Cam Number`))))

(fn `SetMeshes`
  (params (MeshType :type "/Game/Blueprints/Datas/Enum/E_MeshType Enum" :default "NewEnumerator0") (StaticMeshes :type "Array of /Game/Blueprints/Datas/Struct/ST_StaticMeshTransform Structure") (SkeletalMeshes :type "Array of /Game/Blueprints/Datas/Struct/ST_SkeletalMeshTransform Structure"))
  (bind _output_get (set `self.Mesh Type` MeshType))
  (switch `/Game/Blueprints/Datas/Enum/E_MeshType` _output_get
    (:`NewEnumerator0`
      (`self.SetStaticMeshComp` StaticMeshes))
    (:`NewEnumerator1`
      (`self.SetSkeletalMeshComp` SkeletalMeshes))))

(fn `SetSkeletalMeshComp`
  (params (SkeletalMeshes :type "Array of /Game/Blueprints/Datas/Struct/ST_SkeletalMeshTransform Structure"))
  (for _array_element SkeletalMeshes
    (bind (_skeletalmesh _transform) (break `/Game/Blueprints/Datas/Struct/ST_SkeletalMeshTransform` _array_element))
    (bind _returnvalue (`AddComponent|NODE_AddSkeletalMeshComponent-0` :`RelativeTransform` _transform))
    (`KismetArrayLibrary.Array_Add` (`self.SkeletalMeshesComp`) _returnvalue)
    (`SkeletalMeshComponent.SetSkeletalMeshAsset` _returnvalue _skeletalmesh)))

(fn `SetStaticMeshComp`
  (params (StaticMeshes :type "Array of /Game/Blueprints/Datas/Struct/ST_StaticMeshTransform Structure"))
  (for _array_element StaticMeshes
    (bind (_staticmesh _transform) (break `/Game/Blueprints/Datas/Struct/ST_StaticMeshTransform` _array_element))
    (bind _returnvalue (`AddComponent|NODE_AddStaticMeshComponent-0` :`RelativeTransform` _transform))
    (`KismetArrayLibrary.Array_Add` (`self.StaticMeshesComp`) _returnvalue)
    (`StaticMeshComponent.SetStaticMesh` _returnvalue _staticmesh)))

(fn `UserConstructionScript`)