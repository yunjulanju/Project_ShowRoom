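; BP_ShowRoomClothesManager spawns the clothing displays in the showroom from a data table when play begins.
; It loops over every table row and spawns a BP_ShowRoomClothes actor at the row's transform with the product name, owned by the manager.
; Each spawned actor then receives the row's mannequin, interactable setting and product list through SetProductInfo.
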(event `self.ReceiveBeginPlay`
  (bind _outrownames (`DataTableFunctionLibrary.GetDataTableRowNames` (`self.Table`)))
  (for _array_element _outrownames
    (bind _returnvalue (`|GetDataTableRow` (`self.Table`) _array_element)
      (:`then`
        (`self.SpawnProductObjects` _returnvalue)))))

(fn `SpawnProductObjects`
  (params (`Out Row` :type "/Game/Blueprints/Datas/Struct/ST_Fashion_ShowRoom Structure"))
  (bind (_productname _mannequin _interactionable _transform _products) (break `/Game/Blueprints/Datas/Struct/ST_Fashion_ShowRoom` `Out Row`))
  (bind _returnvalue (`|SpawnActorFromClass` "/Game/Blueprints/ShowRoom/BP_ShowRoomClothes.BP_ShowRoomClothes_C" _transform "AlwaysSpawn" "MultiplyWithRoot" self _productname null))
  (`/Game/Blueprints/ShowRoom/BP_ShowRoomClothes.SetProductInfo` _returnvalue _mannequin _interactionable _products))

(fn `UserConstructionScript`)