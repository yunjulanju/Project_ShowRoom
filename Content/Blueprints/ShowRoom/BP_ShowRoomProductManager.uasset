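; Showroom manager actor that populates the level with products defined in a data table.
; On BeginPlay it iterates every row of the table and spawns a BP_Product at the row's transform, owned by the manager.
; Each product receives its name and interactable flag on spawn, then its static or skeletal meshes through SetMeshes according to the row's mesh type.
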(event `self.ReceiveBeginPlay`
  (bind _outrownames (`DataTableFunctionLibrary.GetDataTableRowNames` (`self.Table`)))
  (for _array_element _outrownames
    (bind _returnvalue (`|GetDataTableRow` (`self.Table`) _array_element)
      (:`then`
        (`self.SpawnProductObjects` _returnvalue)))))

(fn `SpawnProductObjects`
  (params (`Out Row` :type "/Game/Blueprints/Datas/Struct/ST_Product Structure"))
  (bind (_productname _bisinteractable _transform _meshtype _staticmesh _skeletalmesh) (break `/Game/Blueprints/Datas/Struct/ST_Product` `Out Row`))
  (bind _returnvalue (`|SpawnActorFromClass` "/Game/Blueprints/ShowRoom/BP_Product.BP_Product_C" _transform "Undefined" "MultiplyWithRoot" self _productname _bisinteractable null))
  (`/Game/Blueprints/ShowRoom/BP_Product.SetMeshes` _returnvalue _meshtype _staticmesh _skeletalmesh))

(fn `UserConstructionScript`)