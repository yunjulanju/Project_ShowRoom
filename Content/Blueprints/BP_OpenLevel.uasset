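; BP_OpenLevel is a level portal that loads the level named in LevelName when a BP_Character stays in its Box trigger.
; On BeginPlay, its Widget component's WBP_MoveLevelInfo displays that level name.
; Overlap begin sets IsOverlap and starts a two-second timer, whose MoveLevel event opens the level only if IsOverlap is still true.
; Overlap end clears the flag but leaves the timer running.
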(event `self.ReceiveBeginPlay`
  (bind _aswbp_move_level_info (cast `/Game/UI/WBP_MoveLevelInfo` (`WidgetComponent.GetUserWidgetObject` (`self.Widget`))))
  (set `TextBlock.Text` (`KismetTextLibrary.Conv_NameToText` (`self.Level Name`)) (`/Game/UI/WBP_MoveLevelInfo.LevelName_txt` _aswbp_move_level_info)))

(event `self.Box.OnComponentBeginOverlap`
  (params (OverlappedComponent :type "PrimitiveComponent Object Reference") (OtherActor :type "Actor Object Reference") (OtherComp :type "PrimitiveComponent Object Reference") (OtherBodyIndex :type Integer) (bFromSweep :type Boolean) (SweepResult :type "HitResult Structure (by ref)"))
  (cast `/Game/Blueprints/Character/BP_Character` OtherActor)
  (set `self.bIsOverlap` true)
  (`KismetSystemLibrary.K2_SetTimerDelegate` (delegate `MoveLevel`) 2.0))

(event `MoveLevel`
  (if (`self.bIsOverlap`)
    (`GameplayStatics.OpenLevel` (`self.Level Name`))
    (set `self.bIsOverlap` false)))

(event `self.Box.OnComponentEndOverlap`
  (params (OverlappedComponent :type "PrimitiveComponent Object Reference") (OtherActor :type "Actor Object Reference") (OtherComp :type "PrimitiveComponent Object Reference") (OtherBodyIndex :type Integer))
  (cast `/Game/Blueprints/Character/BP_Character` OtherActor)
  (set `self.bIsOverlap` false))

(fn `UserConstructionScript`)