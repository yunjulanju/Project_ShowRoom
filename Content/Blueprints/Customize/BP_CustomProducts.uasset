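; BP_CustomProducts is a display product for character customization that the player equips by standing in its trigger box.
; AddProduct stores the product struct and spawns a skeletal mesh component that shows its mesh with a looping idle animation.
; A BP_Character overlap starts a two-second timer, which passes the product to EquipMesh if the overlap flag is still set.
; Leaving the box clears that flag but not the timer.
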(event `self.Box.OnComponentBeginOverlap`
  (params (OverlappedComponent :type "PrimitiveComponent Object Reference") (OtherActor :type "Actor Object Reference") (OtherComp :type "PrimitiveComponent Object Reference") (OtherBodyIndex :type Integer) (bFromSweep :type Boolean) (SweepResult :type "HitResult Structure (by ref)"))
  (bind _asbp_character (cast `/Game/Blueprints/Character/BP_Character` OtherActor))
  (set `self.bIsOverlap` true)
  (`KismetSystemLibrary.K2_SetTimerDelegate` (delegate `SendProductInfo`) 2.0))

(event `SendProductInfo`
  (if (`self.bIsOverlap`)
    (`/Game/Blueprints/Character/BP_Character.EquipMesh` (stale `self.Box.OnComponentBeginOverlap` _asbp_character) (`self.ST Products`))
    (set `self.bIsOverlap` false)))

(event `self.Box.OnComponentEndOverlap`
  (params (OverlappedComponent :type "PrimitiveComponent Object Reference") (OtherActor :type "Actor Object Reference") (OtherComp :type "PrimitiveComponent Object Reference") (OtherBodyIndex :type Integer))
  (cast `/Game/Blueprints/Character/BP_Character` OtherActor)
  (set `self.bIsOverlap` false))

(fn `AddProduct`
  (params (ST_Products :type "/Game/Blueprints/Datas/Struct/Customizing/ST_CustomizeProduct Structure"))
  (locals (OldSkeletalMeshesMap :type "Map of SkeletalMeshComponent Object Reference to /Game/Blueprints/Datas/Enum/E_CustomizeType Enum"))
  (bind _output_get (set `self.ST Products` ST_Products))
  (bind _returnvalue (`AddComponent|NODE_AddSkeletalMeshComponent-0` :`RelativeTransform` (`KismetMathLibrary.MakeTransform` (`SceneComponent.RelativeLocation` (`self.SkeletalMesh`)))))
  (`SkeletalMeshComponent.SetSkeletalMeshAsset` _returnvalue (`.Mesh_2_D6229A134D32DA35DC2AE9BF63F6A86F` (break `/Game/Blueprints/Datas/Struct/Customizing/ST_CustomizeProduct` _output_get)))
  (`SkeletalMeshComponent.PlayAnimation` _returnvalue "/Game/Creative_Characters_FREE/Animations/ANIM_Idle_Breathing.ANIM_Idle_Breathing" true))

(fn `UserConstructionScript`)