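; BP_CustomizeItemManager is an actor that spawns and fills a row of customization product displays.
; On BeginPlay it spawns BP_CustomProducts actors, alternating either side of itself along Y.
; It then filters DT_CustomizeProducts rows by matching a column's text to its ItemType variable, ignoring the passed "Face" argument.
; Each matching row's mesh and type go to the product actor at the same index.
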(event `self.ReceiveBeginPlay`
  (`self.CreateCustomProducts`)
  (bind _outrownames (`DataTableFunctionLibrary.GetDataTableRowNames` "/Game/Blueprints/Datas/DataTable/Customize/DT_CustomizeProducts.DT_CustomizeProducts"))
  (set `self.Out Row Names` _outrownames)
  (bind _findrownames (`self.GetItemTypeRowName` "ItemType" "Face"))
  (for (_array_element _array_index) _findrownames
    (bind _returnvalue (`|GetDataTableRow` "/Game/Blueprints/Datas/DataTable/Customize/DT_CustomizeProducts.DT_CustomizeProducts" _array_element)
      (:`then`
        (bind (_mesh _itemtype) (break `/Game/Blueprints/Datas/Struct/Customizing/ST_CustomizeProduct` _returnvalue))
        (`/Game/Blueprints/Customize/BP_CustomProducts.AddProduct` (`|GetArrayItem` (`self.CustomProducts`) _array_index) _mesh _itemtype)))))

(fn `CreateCustomProducts`
  (bind (_returnvalue_x _returnvalue_y _returnvalue_z) (`KismetMathLibrary.BreakVector` (`self.K2_GetActorLocation`)))
  (for _index (range 1 (+ (`self.MaxIndex`) 1))
    (bind _returnvalue (`|SpawnActorFromClass` "/Game/Blueprints/Customize/BP_CustomProducts.BP_CustomProducts_C" (`KismetMathLibrary.MakeTransform` (`KismetMathLibrary.MakeVector` _returnvalue_x (+ (* (/ _index 2) (select `int` (mod _index 2) :`0` 1 :`1` -1) 150) _returnvalue_y) _returnvalue_z) (`self.K2_GetActorRotation`)) "Undefined" "MultiplyWithRoot" null null))
    (`KismetArrayLibrary.Array_Add` (`self.CustomProducts`) _returnvalue)))

(fn `GetItemTypeRowName`
  (params (InItemType :type Name) (FindType :type String))
  (returns (FindRowNames :type "Array of Name"))
  (locals (FindRowNameArray :type "Array of Name"))
  (bind _returnvalue (`DataTableFunctionLibrary.GetDataTableColumnAsString` "/Game/Blueprints/Datas/DataTable/Customize/DT_CustomizeProducts.DT_CustomizeProducts" InItemType))
  (for (_array_element _array_index) _returnvalue
    (if (`KismetStringLibrary.Contains` _array_element (`|GetEnumeratorNameAsString` (`self.ItemType`)))
      (`KismetArrayLibrary.Array_Add` (`local.FindRowNameArray`) (`|GetArrayItem` (`self.Out Row Names`) _array_index))))
  (return (`local.FindRowNameArray`)))

(fn `UserConstructionScript`)