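; Manager actor for the fashion show room that presents products in sequence from the DT_FashionShowInfo data table.
; On BeginPlay it caches the row names and spawns a BP_FashionShowProduct at the first row's first waypoint, passing it the row data.
; It binds to each product's point-arrive event, and ProductFinish advances the index to spawn the next row until the table is exhausted.
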(event `ProductFinish`
  (bind _output_get (set `self.CurrentIndex` (+ (`self.CurrentIndex`) 1)))
  (if (< _output_get (`self.Index`))
    (`self.SetFashionShowInfo`)))

(event `self.ReceiveBeginPlay`
  (bind _outrownames (`DataTableFunctionLibrary.GetDataTableRowNames` "/Game/Blueprints/Datas/DataTable/FashionShow/DT_FashionShowInfo.DT_FashionShowInfo"))
  (bind _output_get (set `self.Out Row Names` _outrownames))
  (set `self.Index` (`KismetArrayLibrary.Array_Length` _output_get))
  (`self.SetFashionShowInfo`))

(fn `SetFashionShowInfo`
  (bind _returnvalue (`|GetDataTableRow` "/Game/Blueprints/Datas/DataTable/FashionShow/DT_FashionShowInfo.DT_FashionShowInfo" (`|GetArrayItem` (`self.Out Row Names`) (`self.CurrentIndex`)))
    (:`then`
      (`self.SpawnProductInfo` _returnvalue))))

(fn `SpawnProductInfo`
  (params (InRow :type "/Game/Blueprints/Datas/Struct/ST_FashionShowInfo Structure"))
  (bind _returnvalue (`|SpawnActorFromClass` "/Game/Blueprints/FashionShowRoom/BP_FashionShowProduct.BP_FashionShowProduct_C" (`.WayPoint_2_AAEA2E0248CEC355916F0DBB8AF00209` (break `/Game/Blueprints/Datas/Struct/ST_WaypointTime` (`|GetArrayItem` (`.WayPoints_19_7B6F3A264D471F6F7E66158A2E32A59D` (break `/Game/Blueprints/Datas/Struct/ST_FashionShowInfo` InRow))))) "Undefined" "MultiplyWithRoot" null null))
  (`/Game/Blueprints/FashionShowRoom/BP_FashionShowProduct.SetInfo` _returnvalue InRow)
  (add `/Game/Blueprints/FashionShowRoom/BP_FashionShowProduct.PointArrive` _returnvalue (`|CreateDelegate` :!event `ProductFinish`)))

(fn `UserConstructionScript`)