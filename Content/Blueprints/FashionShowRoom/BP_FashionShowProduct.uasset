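; Fashion show product actor that displays a set of meshes and carries them along a waypoint path.
; SetInfo builds static mesh components from the supplied info and stores its waypoints and cameras.
; Tick moves at constant speed toward each waypoint, snapping to its rotation and waiting its set time on arrival.
; Past the last waypoint, every Tick runs ClearStaticMeshComponents, which destroys the meshes and calls PointArrive.
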(event `self.ReceiveBeginPlay`)

(event `self.ReceiveTick`
  (params (DeltaSeconds :type "Float (single-precision)"))
  (bind (_waypoint _movetime _waittime) (break `/Game/Blueprints/Datas/Struct/FashionShow/ST_WaypointTime` (`|GetArrayItem` (`self.Way Points`) (`self.Index`))))
  (if (< (`self.Index`) (`self.IndexLength`))
    (if (<= (`KismetMathLibrary.VSize` (- (.location _waypoint) (`self.K2_GetActorLocation`))) 50.0)
      (`KismetSystemLibrary.Delay` _waittime)
      (`/Engine/EditorBlueprintResources/StandardMacros.IncrementInt` (`self.Index`))
      (else
        (`self.K2_SetActorLocationAndRotation` (`KismetMathLibrary.VInterpTo_Constant` (`self.K2_GetActorLocation`) (.location _waypoint) (`GameplayStatics.GetWorldDeltaSeconds`) 500.0) (.rotation _waypoint))))
    (else
      (`self.ClearStaticMeshComponents`))))

(fn `ClearStaticMeshComponents`
  (for _array_element (`self.StaticMeshComponents`)
    (`ActorComponent.K2_DestroyComponent` _array_element))
  (`KismetArrayLibrary.Array_Clear` (`self.StaticMeshComponents`))
  (`self.PointArrive`))

(fn `SetInfo`
  (params (Info :type "/Game/Blueprints/Datas/Struct/FashionShow/ST_FashionShowInfo Structure"))
  (bind (_brandname _outfitnumber _meshes _waypoints _camera) (break `/Game/Blueprints/Datas/Struct/FashionShow/ST_FashionShowInfo` Info))
  (`|ExecutionSequence`
    (:`then_0`
      (for _array_element _meshes
        (bind _returnvalue (`AddComponent|NODE_AddStaticMeshComponent-0` :`RelativeTransform` (`.Transform_6_33D266764536582172C891A6AD269446` (break `/Game/Blueprints/Datas/Struct/ST_Transform` _array_element))))
        (`KismetArrayLibrary.Array_Add` (`self.StaticMeshComponents`) _returnvalue)
        (`StaticMeshComponent.SetStaticMesh` _returnvalue (break `/Game/Blueprints/Datas/Struct/ST_Transform` _array_element))))
    (:`then_1`
      (bind _output_get (set `self.Way Points` _waypoints))
      (set `self.IndexLength` (`KismetArrayLibrary.Array_Length` _output_get))
      (set `self.Index` 0))
    (:`then_2`
      (set `self.Cameras` _camera))))

(fn `UserConstructionScript`)