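; BP_CharacterController is a player controller that routes movement and look input to the possessed BP_Character.
; On possess it caches the cast pawn and enables movement through SetMove.
; While the IsMove flag is on, axis inputs drive Move and Turn on the character.
; When it is off, movement input is ignored and Turn and LookUp rotate a product through RotateProduct instead.
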(event `self.ReceivePossess`
  (params (PossessedPawn :type "Pawn Object Reference"))
  (bind _asbp_character (cast `/Game/Blueprints/Character/BP_Character` PossessedPawn))
  (set `self.As BP Character` _asbp_character)
  (`self.SetMove` true))

(event `InputAxis|Forward`
  (params (AxisValue :type "Float (single-precision)"))
  (if (`self.bIsMove`)
    (`/Game/Blueprints/Character/BP_Character.Move` (`self.As BP Character`) AxisValue true)))

(event `InputAxis|Right`
  (params (AxisValue :type "Float (single-precision)"))
  (if (`self.bIsMove`)
    (`/Game/Blueprints/Character/BP_Character.Move` (`self.As BP Character`) AxisValue false)))

(event `InputAxis|Turn`
  (params (AxisValue :type "Float (single-precision)"))
  (bind _as_bp_character (`self.As BP Character`))
  (if (`self.bIsMove`)
    (`/Game/Blueprints/Character/BP_Character.Turn` _as_bp_character AxisValue false)
    (else
      (`/Game/Blueprints/Character/BP_Character.RotateProduct` _as_bp_character AxisValue false))))

(event `InputAxis|LookUp`
  (params (AxisValue :type "Float (single-precision)"))
  (bind _as_bp_character (`self.As BP Character`))
  (if (`self.bIsMove`)
    (`/Game/Blueprints/Character/BP_Character.Turn` _as_bp_character AxisValue true)
    (else
      (`/Game/Blueprints/Character/BP_Character.RotateProduct` _as_bp_character AxisValue true))))

(fn `SetMove`
  (params (NewMove :type Boolean))
  (set `self.bIsMove` NewMove))

(fn `UserConstructionScript`)