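; Player character for a product showroom that walks, looks around and inspects nearby BP_ShowRoomProduct actors.
; Capsule overlaps track the current product and whether interaction is allowed, enabling axis-driven rotation of products flagged as interactable.
; SetTargetCameraComponent toggles a blended view target between character and product, disabling movement through BP_CharacterController during inspection and resetting the product's rotation on return.
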(event `self.ReceiveBeginPlay`
  (bind _asbp_character_controller (cast `/Game/Blueprints/Character/BP_CharacterController` (`GameplayStatics.GetPlayerController` 0)))
  (set `self.Character Controller` _asbp_character_controller))

(event `self.CapsuleComponent.OnComponentBeginOverlap`
  (params (OverlappedComponent :type "PrimitiveComponent Object Reference") (OtherActor :type "Actor Object Reference") (OtherComp :type "PrimitiveComponent Object Reference") (OtherBodyIndex :type Integer) (bFromSweep :type Boolean) (SweepResult :type "HitResult Structure (by ref)"))
  (bind _asbp_show_room_product (cast `/Game/Blueprints/ShowRoom/BP_ShowRoomProduct` OtherActor)
    (:`then`
      (set `self.BP Show Room Product` _asbp_show_room_product)
      (set `self.bCanInteract` true))
    (:`CastFailed`
      (set `self.BP Show Room Product` null))))

(event `self.CapsuleComponent.OnComponentEndOverlap`
  (params (OverlappedComponent :type "PrimitiveComponent Object Reference") (OtherActor :type "Actor Object Reference") (OtherComp :type "PrimitiveComponent Object Reference") (OtherBodyIndex :type Integer))
  (set `self.BP Show Room Product` null)
  (set `self.bCanInteract` false))

(fn `Move`
  (params (InValue :type "Float (double-precision)") (bIsForward :type Boolean))
  (if bIsForward
    (`self.AddMovementInput` (`self.GetActorForwardVector`) InValue)
    (else
      (`self.AddMovementInput` (`self.GetActorRightVector`) InValue))))

(fn `RotateProduct`
  (params (AxisValue :type "Float (double-precision)") (bIsX :type Boolean))
  (bind _bp_show_room_product (`self.BP Show Room Product`))
  (bind _bisinteractionable (`/Game/Blueprints/ShowRoom/BP_ShowRoomProduct.bIsInteractionable` _bp_show_room_product))
  (if (`self.bCanInteract`)
    (`/Engine/EditorBlueprintResources/StandardMacros.IsValid` (`self.BP Show Room Product`)
      (:`Is Valid`
        (if (`local.bIsX`)
          (`/Engine/EditorBlueprintResources/StandardMacros.IsValid` _bp_show_room_product
            (:`Is Valid`
              (if _bisinteractionable
                (`/Game/Blueprints/ShowRoom/BP_ShowRoomProduct.MouseRotate` (`self.BP Show Room Product`) (`KismetMathLibrary.MakeRotator` (* (`local.AxisValue`) 1.5))))))
          (else
            (`/Engine/EditorBlueprintResources/StandardMacros.IsValid` _bp_show_room_product
              (:`Is Valid`
                (if _bisinteractionable
                  (`/Game/Blueprints/ShowRoom/BP_ShowRoomProduct.MouseRotate` (`self.BP Show Room Product`) (`KismetMathLibrary.MakeRotator` 0.0 0.0 (* (`local.AxisValue`) 1.5))))))))))))

(fn `SetTargetCameraComponent`
  (returns (TargetActor :type "/Game/Blueprints/ShowRoom/BP_ShowRoomProduct Object Reference"))
  (bind _character_controller (`self.Character Controller`))
  (bind _character_controller_2 (`self.Character Controller`))
  (bind _bp_show_room_product (`self.BP Show Room Product`))
  (`/Engine/EditorBlueprintResources/StandardMacros.IsValid` _bp_show_room_product
    (:`Is Valid`
      (if (`/Game/Blueprints/ShowRoom/BP_ShowRoomProduct.bInPlayer` _bp_show_room_product)
        (if (`self.bChangedView`)
          (set `self.bChangedView` false)
          (`PlayerController.SetViewTargetWithBlend` _character_controller self 0.5 "VTBlend_Linear" 0.0 false)
          (`/Game/Blueprints/Character/BP_CharacterController.SetMove` _character_controller true)
          (`/Game/Blueprints/ShowRoom/BP_ShowRoomProduct.InitMeshRotate` (`self.BP Show Room Product`))
          (return null)
          (else
            (set `self.bChangedView` true)
            (`PlayerController.SetViewTargetWithBlend` _character_controller_2 (`self.BP Show Room Product`) 0.5 "VTBlend_Linear" 0.0 false)
            (`/Game/Blueprints/Character/BP_CharacterController.SetMove` _character_controller_2 false)
            (return (`self.BP Show Room Product`))))))))

(fn `Turn`
  (params (InValue :type "Float (double-precision)") (bIsPitch :type Boolean))
  (if bIsPitch
    (`self.AddControllerPitchInput` InValue)
    (else
      (`self.AddControllerYawInput` InValue))))

(fn `UserConstructionScript`)