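; Player character for the showroom that lets the player interact with BP_ShowRoomProduct actors.
; Capsule overlap events track a single current product, clearing it when any overlap ends or a non-product begins overlapping.
; Pressing the Interaction input calls PossessCamera on that product if it is valid and its InPlayer flag is set.
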(event `self.ReceiveActorBeginOverlap`
  (params (OtherActor :type "Actor Object Reference")))

(event `InputAction|Interaction`
  (params (Key :type "Key Structure"))
  (bind _as_bp_show_room_product (`self.As BP Show Room Product`))
  (:`Pressed`
    (`/Engine/EditorBlueprintResources/StandardMacros.IsValid` _as_bp_show_room_product
      (:`Is Valid`
        (if (`/Game/Blueprints/ShowRoom/BP_ShowRoomProduct.bInPlayer` _as_bp_show_room_product)
          (`/Game/Blueprints/ShowRoom/BP_ShowRoomProduct.PossessCamera` (`self.As BP Show Room Product`)))))))

(event `self.CapsuleComponent.OnComponentBeginOverlap`
  (params (OverlappedComponent :type "PrimitiveComponent Object Reference") (OtherActor :type "Actor Object Reference") (OtherComp :type "PrimitiveComponent Object Reference") (OtherBodyIndex :type Integer) (bFromSweep :type Boolean) (SweepResult :type "HitResult Structure (by ref)"))
  (bind _asbp_show_room_product (cast `/Game/Blueprints/ShowRoom/BP_ShowRoomProduct` OtherActor)
    (:`then`
      (set `self.As BP Show Room Product` _asbp_show_room_product))
    (:`CastFailed`
      (set `self.As BP Show Room Product` null))))

(event `self.CapsuleComponent.OnComponentEndOverlap`
  (params (OverlappedComponent :type "PrimitiveComponent Object Reference") (OtherActor :type "Actor Object Reference") (OtherComp :type "PrimitiveComponent Object Reference") (OtherBodyIndex :type Integer))
  (set `self.As BP Show Room Product` null))

(fn `UserConstructionScript`)