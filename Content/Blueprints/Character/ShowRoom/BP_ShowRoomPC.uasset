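; Player controller for the showroom that lets the player switch camera views on an interaction target.
; On BeginPlay it casts the inherited character reference to BP_ShowRoomCharacter and caches it.
; The Interaction input stores the target returned by the character's SetTargetCameraComponent, and RightMove and LeftMove step that target's camera number in either direction.
; The SetMove override only calls the parent.
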(event `self.ReceiveBeginPlay`
  (bind _as_bp_character (`self.As BP Character`))
  (`/Engine/EditorBlueprintResources/StandardMacros.IsValid` _as_bp_character
    (:`Is Valid`
      (bind _asbp_show_room_character (cast `/Game/Blueprints/Character/ShowRoom/BP_ShowRoomCharacter` _as_bp_character))
      (set `self. BP Show Room Character` _asbp_show_room_character))))

(event `InputAction|Interaction`
  (params (Key :type "Key Structure"))
  (:`Pressed`
    (bind _targetactor (`/Game/Blueprints/Character/ShowRoom/BP_ShowRoomCharacter.SetTargetCameraComponent` (`self. BP Show Room Character`)))
    (set `self.Target Actor` _targetactor)))

(event `InputAction|RightMove`
  (params (Key :type "Key Structure"))
  (bind _target_actor (`self.Target Actor`))
  (:`Pressed`
    (`/Engine/EditorBlueprintResources/StandardMacros.IsValid` _target_actor
      (:`Is Valid`
        (`/Game/Blueprints/ShowRoom/BP_ShowRoomProduct.MoveCamNumber` _target_actor true)))))

(event `InputAction|LeftMove`
  (params (Key :type "Key Structure"))
  (bind _target_actor (`self.Target Actor`))
  (:`Pressed`
    (`/Engine/EditorBlueprintResources/StandardMacros.IsValid` _target_actor
      (:`Is Valid`
        (`/Game/Blueprints/ShowRoom/BP_ShowRoomProduct.MoveCamNumber` _target_actor false)))))

(fn `SetMove`
  (params (NewMove :type Boolean))
  (`parent.SetMove` NewMove))

(fn `UserConstructionScript`)